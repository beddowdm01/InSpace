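; Robot AI character Blueprint whose attack fires a laser from its weapon.
; CustomAttack spawns a scaled-down BB_Laser at the weapon mesh's Muzzle socket, matching the socket's rotation and ignoring spawn collisions.
; The event graph holds only disabled stub events, and the construction script just calls the parent.
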(fn `CustomAttack`
  (bind _weaponmesh (`self.WeaponMesh`))
  (`|SpawnActorFromClass` "/Game/World/WorldItems/Weapons/Bullets/BB_Laser.BB_Laser_C" (`KismetMathLibrary.MakeTransform` (`SceneComponent.GetSocketLocation` _weaponmesh "Muzzle") (`SceneComponent.GetSocketRotation` _weaponmesh "Muzzle") (0.33 0.33 0.33)) "AlwaysSpawn" "OverrideRootScale" null null)
  (return))

(fn `UserConstructionScript`
  (`parent.UserConstructionScript`))