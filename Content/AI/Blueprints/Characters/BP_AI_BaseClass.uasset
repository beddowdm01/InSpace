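; Base AI character class providing shared health, death, patrol and attack logic.
; Damage reduces the health in a stats struct; at zero it flags death, drops an item once and destroys the actor after a delay.
; UseAttack calls CustomAttack and AttackDecision, empty stubs apparently meant for child overrides, then damages the player if approved.
; Helpers set walk speed from crouch/jog state, play attack montages and find or cycle patrol points.
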(event `Event Die`
  (set `self.Attack` false)
  (if (not (`self.Dropped`))
    (`self.DropItem`)
    (set `self.Dropped` true)
    (`KismetSystemLibrary.Delay` 30.0)
    (`self.K2_DestroyActor`)))

(fn `AttackDecision`
  (params (PlayerLoc :type "Vector Structure"))
  (returns (PassDamage :type Boolean))
  (return false))

(fn `ChangePP`
  (if (== (- (`KismetArrayLibrary.Array_Length` (`self.PatrolPoints`)) 1) (`self.FirstPatrolPoint`))
    (set `self.FirstPatrolPoint` 0)
    (else
      (set `self.FirstPatrolPoint` (+ (`self.FirstPatrolPoint`) 1)))))

(fn `CheckDeath`
  (returns (Dead :type Boolean))
  (bind _returnvalue (> (`.Health_2_8E0721544AD9086A1E8EA28BC906D350` (break `/Game/Other/Structs/Character/Struct_Char_Stats` (`self.CharStats`))) 0.0))
  (if (not _returnvalue)
    (bind _retcharbools (`/Game/Other/Function/Libs/BPF_Character.setCharBoolDead` (`self.CharBools`) true))
    (set `self.CharBools` _retcharbools)
    (`self.Event Die`))
  (return _returnvalue))

(fn `CustomAttack`
  (return))

(fn `DropItem`
  (`|SpawnActorFromClass` (`self.ItemToDrop`) (`KismetMathLibrary.MakeTransform` (`self.K2_GetActorLocation`)) "AdjustIfPossibleButAlwaysSpawn" "OverrideRootScale" null null))

(fn `FindClosestPP`
  (returns (NearestIndex :type Integer))
  (locals (NearestLocation :type "Vector Structure") (SmallestDistance :type "Float (double-precision)") (SmallestIndex :type Integer))
  (bind _returnvalue (`self.K2_GetActorLocation`))
  (bind _output_get (set `local.NearestLocation` (`|GetArrayItem` (`self.PatrolPoints`))))
  (set `local.SmallestDistance` (`KismetMathLibrary.VSize` (- _output_get _returnvalue)))
  (for (_array_element _array_index) (`self.PatrolPoints`)
    (bind _returnvalue_2 (`KismetMathLibrary.VSize` (- _array_element _returnvalue)))
    (if (< _returnvalue_2 (`local.SmallestDistance`))
      (set `local.NearestLocation` _array_element)
      (set `local.SmallestDistance` _returnvalue_2)
      (set `local.SmallestIndex` _array_index)))
  (return (`local.SmallestIndex`)))

(fn `OnHit`
  (params (Damage :type "Float (double-precision)"))
  (returns (Dead :type Boolean))
  (bind _dead (`self.TakeDamage` Damage))
  (return _dead))

(fn `PlayAttackMontage`
  (returns (time :type "Float (double-precision)"))
  (bind _returnvalue (`AnimInstance.Montage_Play` (`SkeletalMeshComponent.GetAnimInstance` (`self.Mesh`)) (`self.AttackMontage`) 1.0 "Duration" 0.0))
  (return (- _returnvalue 0.2)))

(fn `SwitchMovementSpeed`
  (params (SwitchInt :type Integer))
  (bind _charactermovement (`self.CharacterMovement`))
  (bind (_standwalkspeed _standrunspeed _standidlejumpvelocity _standmovejumpvelocity _crouchwalkspeed _crouchrunspeed) (break `/Game/Other/Structs/Character/Struct_Char_Movement` (`self.CharMovement`)))
  (bind (_isjogging _iswalking _isjumping _isholdingweapon _iscrouching) (break `/Game/Other/Structs/Character/Struct_Char_Bools` (`self.CharBools`)))
  (switch `int` SwitchInt
    (:`0`
      (if _iscrouching
        (if _isjogging
          (set `CharacterMovementComponent.MaxWalkSpeed` _crouchrunspeed _charactermovement :!label _label)
          (else
            (set `CharacterMovementComponent.MaxWalkSpeed` _crouchwalkspeed _charactermovement)))
        (else
          (set `CharacterMovementComponent.MaxWalkSpeed` _standwalkspeed _charactermovement))))
    (:`1`
      (if _iscrouching
        (goto _label)
        (else
          (set `CharacterMovementComponent.MaxWalkSpeed` _standrunspeed _charactermovement))))))

(fn `TakeDamage`
  (params (DamageAmount :type "Float (double-precision)"))
  (returns (Dead :type Boolean))
  (bind (_health _stamina) (break `/Game/Other/Structs/Character/Struct_Char_Stats` (`self.CharStats`)))
  (bind _returnvalue (- _health DamageAmount))
  (`KismetSystemLibrary.PrintString` (`KismetStringLibrary.Conv_DoubleToString` _returnvalue))
  (set `self.CharStats` (make `/Game/Other/Structs/Character/Struct_Char_Stats` _returnvalue _stamina))
  (bind _dead (`self.CheckDeath`))
  (return _dead))

(fn `UseAttack`
  (params (DamageAmount :type "Float (double-precision)") (PlayerLoc :type "Vector Structure"))
  (returns (Success :type Boolean))
  (`self.CustomAttack`)
  (bind _passdamage (`self.AttackDecision` PlayerLoc))
  (if _passdamage
    (bind _asbp_character_user_01 (cast `/Game/Character/Blueprints/BP_Character_User_01` (`GameplayStatics.GetPlayerPawn` 0)))
    (bind _dead (`/Game/Character/Blueprints/BP_Character_User_01.TakeDamage` _asbp_character_user_01 DamageAmount))
    (set `self.Attack` false)
    (return _dead)))

(fn `UserConstructionScript`)