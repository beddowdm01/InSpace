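; Spider AI character Blueprint that specializes its parent's attack logic with proximity checks on the player's location.
; AttackDecision approves an attack when the player is near the spider, using a vector equality test with a tolerance as a per-axis range check.
; UseAttack applies the same test with a far looser tolerance before deferring to the parent implementation, otherwise returning false.
; BeginPlay and overlap events are unused.
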(fn `AttackDecision`
  (params (PlayerLoc :type "Vector Structure"))
  (returns (PassDamage :type Boolean))
  (return (== PlayerLoc (`self.K2_GetActorLocation`) :`ErrorTolerance` 666.0)))

(fn `UseAttack`
  (params (DamageAmount :type "Float (double-precision)") (PlayerLoc :type "Vector Structure"))
  (returns (Success :type Boolean))
  (if (== PlayerLoc (`self.K2_GetActorLocation`) :`ErrorTolerance` 1000000.0)
    (bind _success (`parent.UseAttack` DamageAmount PlayerLoc))
    (return _success)
    (else
      (return false))))

(fn `UserConstructionScript`
  (`parent.UserConstructionScript`))