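; Behavior tree task that makes an AI character attack, using the pawn of its base AI controller.
; Its Tick event waits briefly, sets the pawn's Attack flag, then delays until shortly before the end of the attack montage's length.
; It then calls UseAttack with the pawn's damage value and the blackboard player location, and finishes successfully.
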(event `self.ReceiveTick`
  (params (OwnerActor :type "Actor Object Reference") (DeltaSeconds :type "Float (single-precision)"))
  (`KismetSystemLibrary.Delay` 0.1)
  (bind _asbp_ai_base_controller (cast `/Game/AI/Blueprints/Controller/BP_AI_BaseController` OwnerActor))
  (bind _asbp_ai_base_class (cast `/Game/AI/Blueprints/Characters/BP_AI_BaseClass` (`Controller.K2_GetPawn` _asbp_ai_base_controller)))
  (set `/Game/AI/Blueprints/Characters/BP_AI_BaseClass.Attack` true _asbp_ai_base_class)
  (bind _returnvalue (`AnimSequenceBase.GetPlayLength` (`/Game/AI/Blueprints/Characters/BP_AI_BaseClass.AttackMontage` _asbp_ai_base_class)))
  (`KismetSystemLibrary.Delay` (- _returnvalue 0.3))
  (`/Game/AI/Blueprints/Characters/BP_AI_BaseClass.UseAttack` _asbp_ai_base_class (`/Game/AI/Blueprints/Characters/BP_AI_BaseClass.AttackDamage` _asbp_ai_base_class) (`BTFunctionLibrary.GetBlackboardValueAsVector` (`self.PlayerLoc`)))
  (`self.FinishExecute` true))