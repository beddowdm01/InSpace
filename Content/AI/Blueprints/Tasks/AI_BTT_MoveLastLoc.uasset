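; Behavior tree task that sends the AI pawn to the player location stored in the blackboard PlayerLoc key.
; If the controller's location is not within tolerance of that point, it sets movement speed mode 0 on the controlled pawn and starts AIMoveTo.
; It finishes successfully as soon as the move is issued, without waiting for arrival.
; When already within tolerance, it never calls FinishExecute.
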(event `self.ReceiveExecute`
  (params (OwnerActor :type "Actor Object Reference"))
  (bind _returnvalue (`BTFunctionLibrary.GetBlackboardValueAsVector` (`self.PlayerLoc`)))
  (bind _asbp_ai_base_controller (cast `/Game/AI/Blueprints/Controller/BP_AI_BaseController` OwnerActor))
  (if (not (== _returnvalue (`Actor.K2_GetActorLocation` _asbp_ai_base_controller) :`ErrorTolerance` 100.0))
    (bind _returnvalue_2 (`Controller.K2_GetPawn` _asbp_ai_base_controller))
    (bind _asbp_ai_base_class (cast `/Game/AI/Blueprints/Characters/BP_AI_BaseClass` _returnvalue_2))
    (`/Game/AI/Blueprints/Characters/BP_AI_BaseClass.SwitchMovementSpeed` _asbp_ai_base_class 0)
    (`|AIMoveTo` _returnvalue_2 _returnvalue null 250.0 true
      (:`then`
        (`self.FinishExecute` true)))))