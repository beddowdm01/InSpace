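; Behavior tree task that sends an AI pawn along its PatrolPoints.
; The first run starts at the closest point and sets the DoneOnce blackboard flag, so later runs start at index zero.
; A custom ForLoopDelay macro waits a fixed delay before each AIMoveTo, which keeps the pawn's current Z.
; Iteration is timer-driven rather than arrival-driven, runs through the array length inclusive, then finishes successfully.
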(event `self.ReceiveExecute`
  (params (OwnerActor :type "Actor Object Reference"))
  (bind _asbp_ai_base_controller (cast `/Game/AI/Blueprints/Controller/BP_AI_BaseController` OwnerActor))
  (bind _returnvalue (`Controller.K2_GetPawn` _asbp_ai_base_controller))
  (bind _asbp_ai_base_class (cast `/Game/AI/Blueprints/Characters/BP_AI_BaseClass` _returnvalue))
  (if (`BTFunctionLibrary.GetBlackboardValueAsBool` (`self.DoneOnce`))
    (set `self.Index` 0)
    (else
      (bind _nearestindex (`/Game/AI/Blueprints/Characters/BP_AI_BaseClass.FindClosestPP` _asbp_ai_base_class))
      (set `self.Index` _nearestindex)
      (`BTFunctionLibrary.SetBlackboardValueAsBool` (`self.DoneOnce`) true)))
  (bind _patrolpoints (`/Game/AI/Blueprints/Characters/BP_AI_BaseClass.PatrolPoints` _asbp_ai_base_class))
  (bind _index (`self.ForLoopDelay` (`self.Index`) (`KismetArrayLibrary.Array_Length` _patrolpoints) :!label _label)
    (:`LoopBody`
      (`|AIMoveTo` _returnvalue (`KismetMathLibrary.MakeVector` (.x (`|GetArrayItem` _patrolpoints _index)) (.y (`|GetArrayItem` _patrolpoints _index)) (.z (`Actor.K2_GetActorLocation` _asbp_ai_base_class))) null -1.0))
    (:`Complete`
      (`self.FinishExecute` true))
    (:`DelayOut`
      (`KismetSystemLibrary.Delay` 15.0)
      (goto _label :!via `DelayIn`))))