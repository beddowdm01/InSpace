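; Behavior tree task that makes an AI search around after it has just lost the player, gated by the JustLostPlayer blackboard flag.
; It sets the AI controller's rotation to the negated stored PlayerRot, then issues random nearby moves around the controller's location.
; A ForLoopDelay macro spaces the moves with delays and clears the flag on completion.
; The task never calls Finish Execute.
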(event `self.ReceiveExecute`
  (params (OwnerActor :type "Actor Object Reference"))
  (if (`BTFunctionLibrary.GetBlackboardValueAsBool` (`self.JustLostPlayer`))
    (bind _asbp_ai_base_controller (cast `/Game/AI/Blueprints/Controller/BP_AI_BaseController` OwnerActor))
    (`Actor.K2_SetActorRotation` _asbp_ai_base_controller (`KismetMathLibrary.NegateRotator` (`BTFunctionLibrary.GetBlackboardValueAsRotator` (`self.PlayerRot`))) false)
    (`self.ForLoopDelay` 0 1 :!label _label
      (:`LoopBody`
        (`|AIMoveTo` (`Controller.K2_GetPawn` _asbp_ai_base_controller) (`KismetMathLibrary.MakeVector` (+ (`KismetMathLibrary.RandomFloatInRange` -500.0 500.0) (.x (`Actor.K2_GetActorLocation` _asbp_ai_base_controller))) (+ (`KismetMathLibrary.RandomFloatInRange` -500.0 500.0) (.y (`Actor.K2_GetActorLocation` _asbp_ai_base_controller))) (.z (`Actor.K2_GetActorLocation` _asbp_ai_base_controller))) null 12.0))
      (:`Complete`
        (`BTFunctionLibrary.SetBlackboardValueAsBool` (`self.JustLostPlayer`)))
      (:`DelayOut`
        (`KismetSystemLibrary.Delay` 3.33)
        (goto _label :!via `DelayIn`)))))