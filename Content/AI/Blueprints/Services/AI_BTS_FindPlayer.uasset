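; Behavior tree service that detects the player for an AI pawn and updates the blackboard, flagging AIDead instead when the pawn is dead.
; A forward sphere trace, then a stationary 750-radius fallback, ignores every actor except the player's pawn and writes sighting, location and rotation keys.
; Without a sighting, it clears focus and attack and yaws the pawn and controller to scan.
; JustLostPlayer delays both steps briefly.
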(event `self.ReceiveTick`
  (params (OwnerActor :type "Actor Object Reference") (DeltaSeconds :type "Float (single-precision)"))
  (bind _asbp_ai_base_controller (cast `/Game/AI/Blueprints/Controller/BP_AI_BaseController` OwnerActor))
  (bind _dead (`self.CheckDead` _asbp_ai_base_controller))
  (if _dead
    (`BTFunctionLibrary.SetBlackboardValueAsBool` (`self.AIDead`) _dead)
    (else
      (if (`BTFunctionLibrary.GetBlackboardValueAsBool` (`self.JustLostPlayer`))
        (`KismetSystemLibrary.Delay` 0.5))
      (`|ExecutionSequence`
        (:`then_0`
          (`self.TracePlayer` _asbp_ai_base_controller))
        (:`then_1`
          (`self.LookAround` _asbp_ai_base_controller DeltaSeconds))))))

(fn `CheckDead`
  (params (AIBaseController :type "AIController Object Reference"))
  (returns (Dead :type Boolean))
  (bind _asbp_ai_base_class (cast `/Game/AI/Blueprints/Characters/BP_AI_BaseClass` (`Controller.K2_GetPawn` AIBaseController)))
  (return (`.isDead_14_57D4BC2C4D009696FB7F3CBE3A58E3AC` (break `/Game/Other/Structs/Character/Struct_Char_Bools` (`/Game/AI/Blueprints/Characters/BP_AI_BaseClass.CharBools` _asbp_ai_base_class)))))

(fn `LookAround`
  (params (AIController :type "/Game/AI/Blueprints/Controller/BP_AI_BaseController Object Reference") (DeltaSeconds :type "Float (double-precision)"))
  (bind _returnvalue (`Controller.K2_GetPawn` AIController))
  (if (not (`BTFunctionLibrary.GetBlackboardValueAsBool` (`self.SeeChar`)))
    (`AIController.K2_SetFocus` AIController null)
    (bind _asbp_ai_base_class (cast `/Game/AI/Blueprints/Characters/BP_AI_BaseClass` _returnvalue))
    (set `/Game/AI/Blueprints/Characters/BP_AI_BaseClass.Attack` false _asbp_ai_base_class)
    (`Actor.K2_SetActorRelativeRotation` _returnvalue (`KismetMathLibrary.MakeRotator` (.roll (`Actor.K2_GetActorRotation` _returnvalue)) (.pitch (`Actor.K2_GetActorRotation` _returnvalue)) (+ (.yaw (`Actor.K2_GetActorRotation` _returnvalue)) 12.5)) false false)
    (`Actor.K2_SetActorRelativeRotation` AIController (`KismetMathLibrary.MakeRotator` (.roll (`Actor.K2_GetActorRotation` _returnvalue)) (.pitch (`Actor.K2_GetActorRotation` _returnvalue)) (+ (.yaw (`Actor.K2_GetActorRotation` _returnvalue)) 12.5)) false false)))

(fn `SetPlayerValues`
  (params (Character :type "/Game/Character/Blueprints/BP_Character_User_01 Object Reference"))
  (`BTFunctionLibrary.SetBlackboardValueAsVector` (`self.PlayerLoc`) (`Actor.K2_GetActorLocation` Character))
  (`BTFunctionLibrary.SetBlackboardValueAsBool` (`self.SeeChar`) true)
  (`BTFunctionLibrary.SetBlackboardValueAsRotator` (`self.PlayerRot`) (`Actor.K2_GetActorRotation` Character)))

(fn `TracePlayer`
  (params (AIController :type "/Game/AI/Blueprints/Controller/BP_AI_BaseController Object Reference"))
  (bind _returnvalue (`Controller.K2_GetPawn` AIController))
  (bind _outactors (`GameplayStatics.GetAllActorsOfClass` "/Script/Engine.Actor"))
  (`KismetArrayLibrary.Array_RemoveItem` _outactors (`Controller.K2_GetPawn` (`GameplayStatics.GetPlayerController` 0)))
  (bind _asbp_ai_base_class (cast `/Game/AI/Blueprints/Characters/BP_AI_BaseClass` _returnvalue))
  (bind _returnvalue_2 (`KismetMathLibrary.MakeVector` (.x (`Actor.K2_GetActorLocation` _returnvalue)) (.y (`Actor.K2_GetActorLocation` _returnvalue)) (+ (.z (`Actor.K2_GetActorLocation` _returnvalue)) (`/Game/AI/Blueprints/Characters/BP_AI_BaseClass.ViewTraceAddHeight` _asbp_ai_base_class))))
  (bind _outhit (`KismetSystemLibrary.SphereTraceSingle` _returnvalue_2 (+ _returnvalue_2 (* (`Actor.GetActorForwardVector` AIController) (`/Game/AI/Blueprints/Characters/BP_AI_BaseClass.ViewTraceDistance` _asbp_ai_base_class))) (`/Game/AI/Blueprints/Characters/BP_AI_BaseClass.ViewSphereTraceSize` _asbp_ai_base_class) "TraceTypeQuery2" false _outactors "None" true (struct :`R` 1.0 :`A` 1.0) (struct :`G` 1.0 :`A` 1.0) 10.0))
  (bind _asbp_character_user_01 (cast `/Game/Character/Blueprints/BP_Character_User_01` (`.HitActor` (`GameplayStatics.BreakHitResult` _outhit)))
    (:`then`
      (`self.SetPlayerValues` _asbp_character_user_01))
    (:`CastFailed`
      (bind _outhit_2 (`KismetSystemLibrary.SphereTraceSingle` _returnvalue_2 _returnvalue_2 750.0 "TraceTypeQuery2" false _outactors))
      (bind _asbp_character_user_01_2 (cast `/Game/Character/Blueprints/BP_Character_User_01` (`.HitActor` (`GameplayStatics.BreakHitResult` _outhit_2)))
        (:`then`
          (`self.SetPlayerValues` _asbp_character_user_01_2))
        (:`CastFailed`
          (`BTFunctionLibrary.SetBlackboardValueAsBool` (`self.SeeChar`)))))))