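; Weapon pickup item Blueprint that shows or removes a weapon mesh on the player's BP_Character_User_01.
; Equip casts the first player's pawn, puts WeaponMesh on its WeaponRef component and stores the mesh-swap result as the hold-weapon flag in CharBools.
; Drop clears that mesh and sets the flag to false.
; Use only defers to the parent, and the event graph has no active logic.
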(fn `Drop`
  (returns (Completed :type Boolean))
  (bind _asbp_character_user_01 (cast `/Game/Character/Blueprints/BP_Character_User_01` (`Controller.K2_GetPawn` (`GameplayStatics.GetPlayerController` 0))))
  (bind _returnvalue (`StaticMeshComponent.SetStaticMesh` (`/Game/Character/Blueprints/BP_Character_User_01.WeaponRef` _asbp_character_user_01) null))
  (bind _retcharbools (`/Game/Other/Function/Libs/BPF_Character.setCharBoolHoldWeapon` (`/Game/Character/Blueprints/BP_Character_User_01.CharBools` _asbp_character_user_01)))
  (set `/Game/Character/Blueprints/BP_Character_User_01.CharBools` _retcharbools _asbp_character_user_01)
  (return _returnvalue))

(fn `Equip`
  (params (NewParam :type Boolean))
  (returns (Completed :type Boolean))
  (bind _asbp_character_user_01 (cast `/Game/Character/Blueprints/BP_Character_User_01` (`Controller.K2_GetPawn` (`GameplayStatics.GetPlayerController` 0))))
  (bind _returnvalue (`StaticMeshComponent.SetStaticMesh` (`/Game/Character/Blueprints/BP_Character_User_01.WeaponRef` _asbp_character_user_01) (`self.WeaponMesh`)))
  (bind _retcharbools (`/Game/Other/Function/Libs/BPF_Character.setCharBoolHoldWeapon` (`/Game/Character/Blueprints/BP_Character_User_01.CharBools` _asbp_character_user_01) _returnvalue))
  (set `/Game/Character/Blueprints/BP_Character_User_01.CharBools` _retcharbools _asbp_character_user_01)
  (return _returnvalue))

(fn `Use`
  (returns (InvClass :type "/Game/Character/Inventory/Items/BP_InventoryActor Class Reference"))
  (bind _invclass (`parent.Use`))
  (return _invclass))

(fn `UserConstructionScript`
  (`parent.UserConstructionScript`))