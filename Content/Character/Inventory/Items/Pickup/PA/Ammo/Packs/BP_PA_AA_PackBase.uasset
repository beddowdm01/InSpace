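; BP_PA_AA_PackBase is the base Blueprint for ammo pack pickups that feed the inventory.
; After the parent construction script runs, it rebuilds the InventoryContents struct with BulletQuant as the quantity.
; Stack limit, inventory class and texture come from the AmmoType class defaults, while display name, type and spawn class keep their existing values.
; The event graph holds only disabled stubs.
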(fn `UserConstructionScript`
  (bind (_displayname _quantity _maxstack _inventoryclass _inventorytype _spawnclass) (break `/Game/Other/Structs/Inventory/Struct_Inv_Item` (`self.InventoryContents`)))
  (bind (_displayname_2 _quantity_2 _maxstack_2 _inventoryclass_2 _inventorytype_2 _spawnclass_2 _inventorytexture) (break `/Game/Other/Structs/Inventory/Struct_Inv_Item` (defaults `Object` (`self.AmmoType`))))
  (`parent.UserConstructionScript`)
  (set `self.InventoryContents` (make `/Game/Other/Structs/Inventory/Struct_Inv_Item` _displayname (`self.BulletQuant`) _maxstack_2 _inventoryclass_2 _inventorytype _spawnclass _inventorytexture)))